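; BP_GameMode is a game mode Blueprint that links the level's enemy to the player controller when play begins.
; It finds all BP_EnemyCharacter actors and stores the first as EnemyInLevel, so it handles a single enemy.
; After a very short delay it casts the first player controller to BP_PlayerController and sets its EnemyTarget to that enemy, with debug prints confirming both steps.
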(event `self.ReceiveBeginPlay`
  (`|ExecutionSequence`
    (:`then_0`
      (bind _outactors (`GameplayStatics.GetAllActorsOfClass` "/Game/Blueprints/Enemy/BP_EnemyCharacter.BP_EnemyCharacter_C"))
      (set `self.EnemyInLevel` (`|GetArrayItem` _outactors))
      (`KismetSystemLibrary.PrintString` "Assigned EnemyCharacter"))
    (:`then_1`
      (`KismetSystemLibrary.Delay` 0.01)
      (bind _asbp_player_controller (cast `/Game/Blueprints/Player/BP_PlayerController` (`GameplayStatics.GetPlayerController` 0)))
      (set `/Game/Blueprints/Player/BP_PlayerController.EnemyTarget` (`self.EnemyInLevel`) _asbp_player_controller)
      (`KismetSystemLibrary.PrintString` "EnemyCh Set!"))))

(fn `UserConstructionScript`)