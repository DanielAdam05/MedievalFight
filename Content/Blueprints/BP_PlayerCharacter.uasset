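; Player character Blueprint that sets up Enhanced Input and moves itself manually each frame.
; BeginPlay adds the default input mapping context to the owning player controller's local subsystem.
; Tick consumes the pending movement input vector, scales it by delta time and MovementSpeed, and applies it as a swept world offset.
; No input actions in this graph feed that vector, and the construction script only calls its parent.
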(event `self.ReceiveBeginPlay`
  (bind _asplayer_controller (cast `PlayerController` (`self.GetController`)))
  (bind _returnvalue (pcsubsystem `EnhancedInputLocalPlayerSubsystem` _asplayer_controller))
  (`/Engine/EditorBlueprintResources/StandardMacros.IsValid` _returnvalue
    (:`Is Valid`
      (`EnhancedInputSubsystemInterface.AddMappingContext` _returnvalue "/Game/Input/IMC_Default.IMC_Default" 0 (struct)))))

(event `self.ReceiveTick`
  (params (DeltaSeconds :type "Float (single-precision)"))
  (bind _returnvalue (`self.ConsumeMovementInputVector`))
  (`self.K2_AddActorWorldOffset` (* (* _returnvalue DeltaSeconds) (`self.MovementSpeed`)) true))

(fn `UserConstructionScript`
  (`parent.UserConstructionScript`))