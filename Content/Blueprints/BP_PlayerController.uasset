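; BP_PlayerController is a player controller that routes Enhanced Input movement and mouse look to the controlled pawn.
; On BeginPlay it registers a mapping context with the local player's Enhanced Input subsystem.
; IA_PlayerMovement swaps the input axes into a length-clamped movement vector along world axes, independent of view rotation.
; IA_MouseLook feeds the controller's yaw and pitch input through the pawn.
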(event `self.ReceiveBeginPlay`
  (bind _returnvalue (subsystem `EnhancedInputLocalPlayerSubsystem`))
  (`/Engine/EditorBlueprintResources/StandardMacros.IsValid` _returnvalue
    (:`Is Valid`
      (`EnhancedInputSubsystemInterface.AddMappingContext` _returnvalue null 0 (struct)))))

(event `EnhancedInput|/Game/Input/IA_PlayerMovement`
  (params (ActionValue :type "Vector2D Structure") (ElapsedSeconds :type "Float (double-precision)") (TriggeredSeconds :type "Float (double-precision)") (InputAction :type "InputAction Object Reference" :default "/Game/Input/IA_PlayerMovement.IA_PlayerMovement"))
  (:`Triggered`
    (`Pawn.AddMovementInput` (`self.K2_GetPawn`) (`KismetMathLibrary.ClampVectorSize` (`KismetMathLibrary.MakeVector` ActionValue_Y ActionValue_X) 0.0 1.0) 1.0 false)))

(event `EnhancedInput|/Game/Input/IA_MouseLook`
  (params (ActionValue :type "Vector2D Structure") (ElapsedSeconds :type "Float (double-precision)") (TriggeredSeconds :type "Float (double-precision)") (InputAction :type "InputAction Object Reference" :default "/Game/Input/IA_MouseLook.IA_MouseLook"))
  (bind _returnvalue (`self.K2_GetPawn`))
  (:`Triggered`
    (`Pawn.AddControllerYawInput` _returnvalue ActionValue_X)
    (`Pawn.AddControllerPitchInput` _returnvalue ActionValue_Y)))

(fn `UserConstructionScript`)