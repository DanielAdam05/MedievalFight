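; BP_PlayerPawn is the player-controlled pawn, handling movement and mouse look through Enhanced Input.
; BeginPlay adds the default mapping context, and the movement action feeds a magnitude-clamped, world-space vector into the pawn's movement input.
; Tick consumes that input and applies a swept offset scaled by MovementSpeed and delta time.
; Mouse look drives controller yaw and pitch, while an actor-rotation lerp sits unconnected and never runs.
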(event `self.ReceiveBeginPlay`
  (bind _asplayer_controller (cast `PlayerController` (`self.GetController`)))
  (bind _returnvalue (pcsubsystem `EnhancedInputLocalPlayerSubsystem` _asplayer_controller))
  (`/Engine/EditorBlueprintResources/StandardMacros.IsValid` _returnvalue
    (:`Is Valid`
      (`EnhancedInputSubsystemInterface.AddMappingContext` _returnvalue "/Game/Input/IMC_Default.IMC_Default" 0 (struct)))))

(event `self.ReceiveTick`
  (params (DeltaSeconds :type "Float (single-precision)"))
  (bind _returnvalue (`self.ConsumeMovementInputVector`))
  (`self.K2_AddActorWorldOffset` (* (* _returnvalue DeltaSeconds) (`self.MovementSpeed`)) true))

(event `EnhancedInput|/Game/Input/IA_PlayerMovement`
  (params (ActionValue :type "Vector2D Structure") (ElapsedSeconds :type "Float (double-precision)") (TriggeredSeconds :type "Float (double-precision)") (InputAction :type "InputAction Object Reference" :default "/Game/Input/IA_PlayerMovement.IA_PlayerMovement"))
  (:`Triggered`
    (`self.AddMovementInput` (`Controller.K2_GetPawn` (`self.GetController`)) (`KismetMathLibrary.ClampVectorSize` (`KismetMathLibrary.MakeVector` ActionValue_Y ActionValue_X) 0.0 1.0) 1.0 false)))

(event `EnhancedInput|/Game/Input/IA_MouseLook`
  (params (ActionValue :type "Vector2D Structure") (ElapsedSeconds :type "Float (double-precision)") (TriggeredSeconds :type "Float (double-precision)") (InputAction :type "InputAction Object Reference" :default "/Game/Input/IA_MouseLook.IA_MouseLook"))
  (:`Triggered`
    (`self.AddControllerYawInput` ActionValue_X)
    (`self.AddControllerPitchInput` ActionValue_Y)))

(fn `UserConstructionScript`)