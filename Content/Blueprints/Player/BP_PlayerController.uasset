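; Player controller that routes Enhanced Input movement and mouse look to the controlled pawn, blocking both when the character's health component reports death.
; BeginPlay caches the player character, adds a mapping context and grabs the level sequence actor at index 1 as the enemy dash sequence.
; Movement uses clamped world axes rather than camera-relative ones.
; Hard-coded keys play that sequence (Space) and toggle mouse look against a cursor with reset view (X).
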(event `Key|SpaceBar`
  (params (Key :type "Key Structure"))
  ; Plays Dash Level Sequence
  (:`Pressed`
    (`/Engine/EditorBlueprintResources/StandardMacros.IsValid` (`self.EnemyDASHSequence`)
      (:`Is Valid`
        (`MovieSceneSequencePlayer.Play` (`LevelSequenceActor.SequencePlayer` (`self.EnemyDASHSequence`))))
      (:`Is Not Valid`
        (`KismetSystemLibrary.PrintString` "\"Enemy Dash Sequence not found\"")))))

(event `self.ReceiveBeginPlay`
  (bind _returnvalue (subsystem `EnhancedInputLocalPlayerSubsystem`))
  ; Get and Set PlayerCharacter
  (`KismetSystemLibrary.Delay` 0.0)
  (bind _asbp_player_character (cast `/Game/Blueprints/Player/BP_PlayerCharacter` (`self.K2_GetPawn`)))
  (set `self.PlayerCharacter` _asbp_player_character)
  (`/Engine/EditorBlueprintResources/StandardMacros.IsValid` _returnvalue
    (:`Is Valid`
      (`EnhancedInputSubsystemInterface.AddMappingContext` _returnvalue null 0 (struct))
      ; Get Enemy Dash Sequence
      (bind _outactors (`GameplayStatics.GetAllActorsOfClass` "/Script/LevelSequence.LevelSequenceActor"))
      (set `self.EnemyDASHSequence` (`|GetArrayItem` _outactors 1)))))

(event `EnhancedInput|/Game/Input/IA_MouseLook`
  (params (ActionValue :type "Vector2D Structure") (ElapsedSeconds :type "Float (double-precision)") (TriggeredSeconds :type "Float (double-precision)") (InputAction :type "InputAction Object Reference" :default "/Game/Input/IA_MouseLook.IA_MouseLook"))
  (bind _returnvalue (`self.K2_GetPawn`))
  ; Mouse Look Logic
  (:`Triggered`
    (if (and (not (`self.IsPlayerCharacterDead`)) (`self.mouseLookEnabled`))
      (`Pawn.AddControllerYawInput` _returnvalue ActionValue_X)
      (`Pawn.AddControllerPitchInput` _returnvalue ActionValue_Y))))

(event `EnhancedInput|/Game/Input/IA_PlayerMovement`
  (params (ActionValue :type "Vector2D Structure") (ElapsedSeconds :type "Float (double-precision)") (TriggeredSeconds :type "Float (double-precision)") (InputAction :type "InputAction Object Reference" :default "/Game/Input/IA_PlayerMovement.IA_PlayerMovement"))
  ; Process Movement Input
  (:`Triggered`
    (if (`self.IsPlayerCharacterDead`)
      (`KismetSystemLibrary.PrintString` "PLAYER IS DEAD")
      (else
        (`Pawn.AddMovementInput` (`self.K2_GetPawn`) (`KismetMathLibrary.ClampVectorSize` (`KismetMathLibrary.MakeVector` ActionValue_Y ActionValue_X) 0.0 1.0) 1.0 false)))))

(event `Key|X`
  (params (Key :type "Key Structure"))
  (:`Pressed`
    (if (not (`self.IsPlayerCharacterDead`))
      ; Sets MouseLookEnabled
      (`/Engine/EditorBlueprintResources/StandardMacros.FlipFlop`
        (:`A`
          (set `self.mouseLookEnabled` true)
          (set `self.bShowMouseCursor` false))
        (:`B`
          (set `self.mouseLookEnabled` false)
          (`self.SetControlRotation` (`self.initialCameraRotation`))
          (set `self.bShowMouseCursor` true))))))

(fn `IsPlayerCharacterDead`
  (returns (IsDead :type Boolean))
  (`/Engine/EditorBlueprintResources/StandardMacros.IsValid` (`self.PlayerCharacter`)
    (:`Is Valid`
      (return (`/Game/Blueprints/Damage/BPC_Health.IsDead` (`/Game/Blueprints/BP_BaseCharacter.BPC_Health` (`self.PlayerCharacter`)))))
    (:`Is Not Valid`
      (`KismetSystemLibrary.PrintString` "BP_PCharacter NOT valid"))))

(fn `UserConstructionScript`)