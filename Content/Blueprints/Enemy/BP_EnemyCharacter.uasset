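; Enemy character Blueprint that plays a death cutscene when its health component reports death.
; On BeginPlay it caches the first LevelSequenceActor found in the level as the death sequence.
; The BPC_Health OnDeath event prints a debug message and plays that sequence, or logs if it is missing.
; Leftover test damage and movement-disable nodes are disconnected and never run.
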(event `self.ReceiveBeginPlay`
  ; Get Enemy Death Sequence
  (bind _outactors (`GameplayStatics.GetAllActorsOfClass` "/Script/LevelSequence.LevelSequenceActor"))
  (set `self.EnemyDeathSequence` (`|GetArrayItem` _outactors)))

(event `self.ReceiveTick`
  (params (DeltaSeconds :type "Float (single-precision)")))

(event `self.BPC_Health.OnDeath`
  (`|ExecutionSequence`
    (:`then_0`
      ; Play Enemy Death Level Sequence
      (`KismetSystemLibrary.PrintString` "ENEMY DEAD")
      (`/Engine/EditorBlueprintResources/StandardMacros.IsValid` (`self.EnemyDeathSequence`)
        (:`Is Valid`
          (`MovieSceneSequencePlayer.Play` (`LevelSequenceActor.SequencePlayer` (`self.EnemyDeathSequence`))))
        (:`Is Not Valid`
          (`KismetSystemLibrary.PrintString` "\"Enemy Death Sequence not found\""))))))

(fn `UserConstructionScript`
  (`parent.UserConstructionScript`))