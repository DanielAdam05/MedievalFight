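; BPC_Health is a health component that tracks current against maximum health and resets it to full on BeginPlay.
; Helper functions derive the health percentage and use it to report death.
; DoDamage clamps health and fires the OnDeath dispatcher if health dropped to zero in that call.
; As written, DoDamage subtracts a constant zero instead of its Amount input, so health never decreases from valid values.
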(event `self.ReceiveBeginPlay`
  (`self.Reset Health`))

(event `/Game/Blueprints/Damage/BPI_Damageable.Reset Health`
  ; Reset Health Implementation
  (set `self.currentHealth` (`self.MaxHealth`)))

(fn `Do Damage`
  (params (Amount :type "Float (double-precision)"))
  (returns (IsDead :type Boolean))
  (locals (originalHealth :type "Float (double-precision)"))
  (bind _currenthealth (`self.currentHealth`))
  ; Deal Damage
  (set `local.originalHealth` _currenthealth)
  (bind _output_get (set `self.currentHealth` (`KismetMathLibrary.FClamp` (- _currenthealth 0.0) 0.0 (`self.MaxHealth`))))
  ; Call OnDeath Event Dispatcher
  (if (and (`self.IsDead`) (> (`local.originalHealth`) _output_get))
    (`self.OnDeath`)
    (return false)))

(fn `GetHealthPercentage`
  (returns (`HP Percentage` :type "Float (double-precision)"))
  (return (/ (`self.currentHealth`) (`self.MaxHealth`))))

(fn `IsDead`
  (returns (IsDead :type Boolean))
  (return (<= (`self.GetHealthPercentage`) 0.0)))